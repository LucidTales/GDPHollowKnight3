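; Player knight for a Hollow Knight-style 2D side-scrolling platformer, with run, double jump, wall slide and jump, dash, and directional nail slashes.
; Custom movement: input, gravity, jump, dash and knockback add acceleration, resolved each Tick through clamped, sliding sweeps that recompute velocity.
; A movement-mode state machine, fed by capsule hits and wall traces, drives limits and flipbooks.
; Slashes message overlapping hitbox actors, triggering knockback on successful side hits.
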(event OnComponentHit(Capsule)
  (params (HitComponent :type Primitive%20Component%20Object%20Reference) (OtherActor :type Actor%20Object%20Reference) (OtherComp :type Primitive%20Component%20Object%20Reference) (NormalImpulse :type Vector :default "0, 0, 0") (Hit :type Hit%20Result%20Structure%20%28by%20ref%29))
  (if (>= (Math|Vector|DotProduct (.normal Hit) "0, 0,1.000000") 0.71)
    (CallFunction|Grounded)
    (elif (>= (Math|Float|Absolute(Float) (Math|Vector|DotProduct (.normal Hit) "0,1.000000,0.000000")) 0.71)
      (Movement|ChangeMovement "NewEnumerator5")
      (Utilities|Time|SetTimerbyFunctionName self "Ungrounded" 1e-06))))

(event OnFinishedPlaying(Slash)
  (Rendering|SetVisibility (Variables|Default|GetDownSlash) false false))

(event OnFinishedPlaying(DownSlash)
  (Rendering|SetVisibility (Variables|Default|GetDownSlash) false false))

(event Custom|Attacking
  (bind _slash (Variables|Default|GetSlash))
  (if (not (Variables|Default|GetbAttacking))
    (Variables|Default|SetbAttacking true)
    (Variables|Default|SetAttackDirection (|AttackDirectionCol))
    (Variables|Default|SetSlashAnim (Utilities|Select :Index (Variables|Default|GetAttackDirection) :NewEnumerator0 "/Game/Sprites/FB_Zote_UpSlash.FB_Zote_UpSlash" :NewEnumerator1 "/Game/Sprites/FB_Zote_DownSlash.FB_Zote_DownSlash" :NewEnumerator2 "/Game/Sprites/FB_Zote_SlashAlt.FB_Zote_SlashAlt" :NewEnumerator3 "/Game/Sprites/FB_Zote_SlashAlt.FB_Zote_SlashAlt"))
    (Rendering|SetVisibility (Utilities|Select :Index (Variables|Default|GetAttackDirection) :NewEnumerator0 (Variables|Default|GetUpSlashFlip) :NewEnumerator1 (Variables|Default|GetDownSlash) :NewEnumerator2 _slash :NewEnumerator3 _slash) true false)
    (Components|Timeline|PlayfromStart (Utilities|Select :Index (Variables|Default|GetAttackDirection) :NewEnumerator0 (Variables|Default|GetUpSlashFlip) :NewEnumerator1 (Variables|Default|GetDownSlash) :NewEnumerator2 _slash :NewEnumerator3 _slash))
    (CallFunction|AttackScan)
    ;[1 1 1] Cooldown
    (Utilities|FlowControl|Delay 0.33333)
    (Variables|Default|SetbAttacking false)))

(event Custom|OnFinishedPlaying%20%28UpSlash%29
  (Rendering|SetVisibility (Variables|Default|GetDownSlash) false false))

(event EventBeginPlay
  (bind _downslash (Variables|Default|GetDownSlash))
  (bind _asbp_flipbook (Utilities|Casting|CastToBP_Flipbook (Variables|/Script/Engine.ChildActorComponent|GetChildActor (Variables|Default|GetChildActor))))
  (Variables|Default|SetFlipbook _asbp_flipbook)
  (bind _asbp_flipbook_2 (Utilities|Casting|CastToBP_Flipbook (Variables|/Script/Engine.ChildActorComponent|GetChildActor (Variables|Default|GetUpSlash))))
  (Variables|Default|SetUpSlashFlip (Variables|/Game/Sprites/BP_Flipbook.BP_Flipbook_C|GetPaperFlipbook _asbp_flipbook_2))
  (Audio|Components|Audio|Stop _downslash)
  (Components|Timeline|SetLooping _downslash false)
  (Rendering|SetVisibility _downslash false false)
  (EventDispatchers|BindEventtoOnFinishedPlaying (Variables|Default|GetUpSlashFlip) (EventDispatchers|CreateEvent :!event Custom|OnFinishedPlaying%20%28UpSlash%29)))

(event EventTick
  (params (DeltaSeconds :type Float%20%28single-precision%29))
  (Utilities|FlowControl|Sequence
    (:then_0
      (Movement|Gravity)
      (Jump|Jumping)
      (Dash|Dashing)
      (Wall|CheckWallCollision))
    (:then_1
      (CallFunction|SetAnim)
      (Knockback|Knockback))
    (:then_2
      (Movement|ResolveMovement))))

(event Input|ActionEvents|InputActionJump
  (params (Key :type Key%20Structure))
  (:Pressed
    (Jump|StartJump))
  (:Released
    (Jump|StopJump true)))

(event Input|ActionEvents|InputActionAttack
  (params (Key :type Key%20Structure))
  (:Pressed
    (CallFunction|Attacking)))

(event Input|ActionEvents|InputActionDash
  (params (Key :type Key%20Structure))
  (:Pressed
    (Dash|StartDash)))

(event Input|AxisEvents|InputAxisRight
  (params (AxisValue :type Float%20%28single-precision%29))
  (bind _returnvalue (Math|Float|Sign(Float) AxisValue))
  (Utilities|FlowControl|Sequence
    (:then_0
      (if (Math|Boolean|ANDBoolean (not (Variables|Knockback|GetbKnockback)) (Utilities|Enum|NotEqual(Enum) (Variables|Movement|GetMovementMode) "NewEnumerator4") (not (Variables|Jump|GetbWallJumpInitial)))
        (Movement|AddVelocity "0.000000,1.000000,0.000000" (* _returnvalue (Variables|Movement|GetMoveRightAccel)))))
    (:then_1
      (if (Variables|Jump|GetbWallJumpInitial)
        (Variables|Default|SetLookDirection (Math|Vector|MakeVector 0.0 _returnvalue 0.0))))))

(fn ConstructionScript)

(fn AddVelocity
  (params (Direcion :type Vector) (Scale :type Float%20%28single-precision%29))
  (Variables|Movement|SetAddedVelocity (+ (* Direcion (* Scale (Utilities|Time|GetWorldDeltaSeconds))) (Variables|Movement|GetAddedVelocity))))

(fn ResolveMovement
  (bind _maxwalkspeed (Variables|Movement|GetMaxWalkSpeed))
  (bind _jumpspeedcap (Variables|Jump|GetJumpSpeedCap))
  (bind _movementmode (Variables|Movement|GetMovementMode))
  (bind _dashmaxspeed (Variables|Dash|GetDashMaxSpeed))
  (bind _movementmode_2 (Variables|Movement|GetMovementMode))
  (bind _maxfallspeed (Variables|Gravity|GetMaxFallSpeed))
  (bind _returnvalue (Utilities|Select :Index _movementmode_2 :NewEnumerator0 _maxwalkspeed :NewEnumerator1 _maxwalkspeed :NewEnumerator3 _maxwalkspeed :NewEnumerator2 _maxwalkspeed :NewEnumerator4 _dashmaxspeed :NewEnumerator5 _maxwalkspeed))
  (LocalVariables|SetLocationBefore (Transformation|GetActorLocation))
  (Utilities|FlowControl|Sequence
    (:then_0
      (bind _sweephitresult (Transformation|SetActorLocation (+ (Transformation|GetActorLocation) (* (Math|Vector|MakeVector 0.0 (Math|Float|Clamp(Float) (|InstantAccel (.Y (Math|Vector|BreakVector (+ (Variables|Movement|GetVelocity) (Variables|Movement|GetAddedVelocity))))) (* _returnvalue -1.0) _returnvalue) (Math|Float|Clamp(Float) (.Z (Math|Vector|BreakVector (+ (Variables|Movement|GetVelocity) (Variables|Movement|GetAddedVelocity)))) (Utilities|Select :Index (Variables|Movement|GetMovementMode) :NewEnumerator0 _maxfallspeed :NewEnumerator1 0.0 :NewEnumerator3 0.0 :NewEnumerator2 _maxfallspeed :NewEnumerator4 0.0 :NewEnumerator5 (select (Variables|Wall|GetbLandedWall) 0.0 (Variables|Wall|GetWallFallSpeed))) (Utilities|Select :Index (Variables|Movement|GetMovementMode) :NewEnumerator0 _jumpspeedcap :NewEnumerator1 _jumpspeedcap :NewEnumerator3 _jumpspeedcap :NewEnumerator2 _jumpspeedcap :NewEnumerator4 0.0 :NewEnumerator5 _jumpspeedcap))) (Utilities|Time|GetWorldDeltaSeconds))) true false))
      (bind _output_get (LocalVariables|SetLocalSweep _sweephitresult))
      ;[1 1 1] Sweep to finish the displacement
      (while (.bBlockingHit (Collision|BreakHitResult _output_get))
        (bind _sweephitresult_2 (Transformation|SetActorLocation (+ (Transformation|GetActorLocation) (- (- (.TraceEnd (Collision|BreakHitResult _output_get)) (.TraceStart (Collision|BreakHitResult _output_get))) (* (.ImpactNormal (Collision|BreakHitResult _output_get)) (Math|Vector|DotProduct (.ImpactNormal (Collision|BreakHitResult _output_get)) (- (.TraceEnd (Collision|BreakHitResult _output_get)) (.TraceStart (Collision|BreakHitResult _output_get))))))) true false))
        (LocalVariables|SetLocalSweep _sweephitresult_2)))
    (:then_1
      (Utilities|FlowControl|Sequence
        (:then_0
          ;[1 1 1] Sets new velocity based on displacement
          (Variables|Movement|SetVelocity (/ (- (Transformation|GetActorLocation) (LocalVariables|GetLocationBefore)) (Utilities|Time|GetWorldDeltaSeconds)))
          (Variables|Movement|SetAddedVelocity "0, 0, 0"))
        (:then_1
          ;[1 1 1] Apex check
          (if (or (Utilities|Enum|Equal(Enum) _movementmode "NewEnumerator1") (Utilities|Enum|Equal(Enum) _movementmode "NewEnumerator3"))
            (if (<= (.z (Variables|Movement|GetVelocity)) 0.0)
              (Movement|ChangeMovement "NewEnumerator2"))))))))

(fn ChangeMovement
  (params (NewMovement :type EMovement%20Enum :default "NewEnumerator0"))
  (LocalVariables|SetOldMovement (Variables|Movement|GetMovementMode))
  (switch Utilities|FlowControl|Switch|SwitchonEMovement NewMovement
    (:NewEnumerator0
      (if (Utilities|Enum|NotEqual(Enum) (Variables|Movement|GetMovementMode) "NewEnumerator4") :!label _label
        (Variables|Movement|SetMovementMode NewMovement :!label _label_2)
        (if (Utilities|Enum|NotEqual(Enum) (LocalVariables|GetOldMovement) NewMovement)
          (Utilities|FlowControl|Sequence
            (:then_0
              (return (Utilities|Enum|NotEqual(Enum) (LocalVariables|GetOldMovement) NewMovement)))
            (:then_1
              (Utilities|FlowControl|Sequence
                (:then_0
                  (switch Utilities|FlowControl|Switch|SwitchonEMovement (LocalVariables|GetOldMovement)
                    (:NewEnumerator5
                      (Variables|Wall|SetbLandedWall false))))
                (:then_1
                  (switch Utilities|FlowControl|Switch|SwitchonEMovement NewMovement
                    (:NewEnumerator5
                      (Variables|Wall|SetbLandedWall true)
                      (Utilities|Time|SetTimerbyFunctionName self "LandedWallFalse" 0.1)))))))
          (else
            (return (Utilities|Enum|NotEqual(Enum) (LocalVariables|GetOldMovement) NewMovement))))))
    (:NewEnumerator1
      (goto _label))
    (:NewEnumerator3
      (goto _label))
    (:NewEnumerator2
      (if (Utilities|Enum|NotEqual(Enum) (Variables|Movement|GetMovementMode) "NewEnumerator1")
        (goto _label_2)))
    (:NewEnumerator4
      (goto _label_2))
    (:NewEnumerator5
      (if (Utilities|Enum|Equal(Enum) (Variables|Movement|GetMovementMode) "NewEnumerator2")
        (goto _label_2)))))

(fn Gravity
  (bind _gravityacceleration (Variables|Gravity|GetGravityAcceleration))
  (Movement|AddVelocity (select (Utilities|Enum|Equal(Enum) (Variables|Movement|GetMovementMode) "NewEnumerator5") (+ "0, 0,-1.000000" (Math|Vector|MakeVector 0.0 (Variables|Wall|GetWallDirection) 0.0)) "0, 0,-1.000000") (Utilities|Select :Index (Variables|Movement|GetMovementMode) :NewEnumerator0 _gravityacceleration :NewEnumerator1 0.0 :NewEnumerator3 (Variables|Gravity|GetRisingGravityAcceleration) :NewEnumerator2 _gravityacceleration :NewEnumerator4 0.0 :NewEnumerator5 _gravityacceleration)))

(fn StartJump
  (if (Utilities|Enum|Equal(Enum) (Variables|Movement|GetMovementMode) "NewEnumerator0")
    (Variables|Jump|SetJumpTimer 0.0 :!label _label)
    (Movement|ChangeMovement "NewEnumerator1")
    (elif (Variables|Wall|GetbTouchingWall)
      (Utilities|FlowControl|Sequence
        (:then_0
          (goto _label))
        (:then_1
          ;[1 1 1] Wall Jump specifics
          (Variables|Jump|SetbWallJumpInitial true)
          (CallFunction|Look (== (Variables|Wall|GetWallDirection) -1.0))
          (Variables|Movement|SetVelocity "0, 0, 0")))
      (else
        ;[1 1 1] Double Jump
        (if (CallFunction|InAir)
          (if (Variables|Jump|GetbDoubleJump)
            (Variables|Jump|SetbDoubleJump false)
            (goto _label)))))))

(fn Jumping
  (if (Utilities|Enum|Equal(Enum) (Variables|Movement|GetMovementMode) "NewEnumerator1")
    (Utilities|FlowControl|Sequence
      (:then_0
        ;[1 1 1] Jump Movement
        (Movement|AddVelocity (select (Variables|Jump|GetbWallJumpInitial) (+ "0, 0,1.000000" (Math|Vector|MakeVector 0.0 (* (Variables|Wall|GetWallDirection) -2.0) 0.0)) "0, 0,1.000000") (Variables|Jump|GetJumpAcceleration)))
      (:then_1
        (Utilities|FlowControl|Sequence
          (:then_0
            ;[1 1 1] Jump Duration
            (bind _output_get (Variables|Jump|SetJumpTimer (+ (Variables|Jump|GetJumpTimer) (Utilities|Time|GetWorldDeltaSeconds))))
            (if (>= _output_get (Variables|Jump|GetJumpMaxDuration))
              (Jump|StopJump false)))
          (:then_1
            ;[1 1 1] Stop jumping away from the wall
            (if (>= (Variables|Jump|GetJumpTimer) (/ (Variables|Jump|GetJumpMaxDuration) 2.0))
              (Variables|Jump|SetbWallJumpInitial false))))))))

(fn StopJump
  (params (bSharp :type Boolean))
  (if (Utilities|Enum|Equal(Enum) (Variables|Movement|GetMovementMode) "NewEnumerator1")
    (Variables|Jump|SetbWallJumpInitial false)
    (Movement|ChangeMovement "NewEnumerator3")
    (if bSharp
      (Movement|AddVelocity "0, 0,-1.000000" (Math|Float|Absolute(Float) (/ (/ (.z (Variables|Movement|GetVelocity)) (Utilities|Time|GetWorldDeltaSeconds)) 1.5))))))

(fn Ungrounded
  (if (not (CallFunction|InAir))
    (Movement|ChangeMovement "NewEnumerator2")))

(fn InAir
  (bind _movementmode (Variables|Movement|GetMovementMode))
  (return (Math|Boolean|ORBoolean (Utilities|Enum|Equal(Enum) _movementmode "NewEnumerator1") (Utilities|Enum|Equal(Enum) _movementmode "NewEnumerator2") (Utilities|Enum|Equal(Enum) _movementmode "NewEnumerator3"))))

(fn SetAnim
  (Utilities|FlowControl|Sequence
    (:then_0
      (if (Math|Boolean|ANDBoolean (not (Variables|Default|GetbAttacking)) (Utilities|Enum|NotEqual(Enum) (Variables|Movement|GetMovementMode) "NewEnumerator4") (not (Variables|Jump|GetbWallJumpInitial)))
        (Math|Float|CompareFloat (Math|Float|Sign(Float) (Input|AxisValues|GetRight)) 0.0
          (:>
            (CallFunction|Look true))
          (:<
            (CallFunction|Look false)))))
    (:then_1
      (Sprite|SetFlipbook (Variables|/Game/Sprites/BP_Flipbook.BP_Flipbook_C|GetPaperFlipbook (Variables|Default|GetFlipbook)) (select (Variables|Default|GetbAttacking) (Variables|Default|GetSlashAnim) (Utilities|Select :Index (Variables|Movement|GetMovementMode) :NewEnumerator0 (select (== (.y (Variables|Movement|GetVelocity)) 0.0) "/Game/Sprites/FB_Zote_IdleWind.FB_Zote_IdleWind" "/Game/Sprites/FB_Zote_Run.FB_Zote_Run") :NewEnumerator1 (select (Variables|Jump|GetbDoubleJump) (select (Variables|Jump|GetbWallJumpInitial) "/Game/Sprites/FB_Zote_Walljump.FB_Zote_Walljump" "/Game/Sprites/FB_Zote_Jump.FB_Zote_Jump") "/Game/Sprites/FB_Zote_DJump.FB_Zote_DJump") :NewEnumerator3 "/Game/Sprites/FB_Zote_Fall.FB_Zote_Fall" :NewEnumerator2 "/Game/Sprites/FB_Zote_Fall.FB_Zote_Fall" :NewEnumerator4 "/Game/Sprites/FB_Zote_Dash.FB_Zote_Dash" :NewEnumerator5 "/Game/Sprites/FB_Zote_Wallslide.FB_Zote_Wallslide"))))))

(fn Look
  (params (Right :type Boolean))
  (Transformation|SetRelativeRotation (Variables|Default|GetChildActor) (Math|Rotator|SelectRotator "0,90.000000, 0" "0,270.000000, 0" Right) false false)
  (Variables|Default|SetLookDirection (select Right "0,1.000000, 0" "0,-1.000000, 0")))

(fn AttackScan
  (bind _slashhitbox (Variables|Default|GetSlashHitbox))
  (LocalVariables|SetAttack (Utilities|Select :Index (Variables|Default|GetAttackDirection) :NewEnumerator0 (Variables|Default|GetUpSlashHitbox) :NewEnumerator1 (Variables|Default|GetDownSlashHitbox) :NewEnumerator2 _slashhitbox :NewEnumerator3 _slashhitbox))
  (Utilities|FlowControl|Sequence
    (:then_0
      (bind _output_get (LocalVariables|SetLocalOverlaps (Collision|GetOverlappingActors (LocalVariables|GetAttack) 0 :!class /Script/Engine.PrimitiveComponent)))
      (for _array_element _output_get
        (bind _bknockback (Class|BPIAttacks|NailAttack(Message) _array_element))
        (if _bknockback
          (LocalVariables|SetHitKnockback true))))
    (:then_1
      (if (LocalVariables|GetHitKnockback)
        (switch Utilities|FlowControl|Switch|SwitchonEDirection (Variables|Default|GetAttackDirection)
          (:NewEnumerator2
            (Knockback|StartKnockback "NewEnumerator3"))
          (:NewEnumerator3
            (Knockback|StartKnockback "NewEnumerator2")))))))

(fn StartKnockback
  (params (KnockbackDirection :type EDirection%20Enum :default "NewEnumerator0"))
  (Variables|Knockback|SetbKnockback true)
  (Variables|Knockback|SetKnockbackDirection KnockbackDirection))

(fn Knockback
  (if (Variables|Knockback|GetbKnockback)
    (Movement|AddVelocity (Utilities|Select :Index (Variables|Knockback|GetKnockbackDirection) :NewEnumerator0 "0, 0,1.000000" :NewEnumerator1 "0, 0, 0" :NewEnumerator2 "0,1.000000, 0" :NewEnumerator3 "0,-1.000000, 0") 3e+03)
    (if (< (Variables|Knockback|GetKnockbackTimer) (Variables|Knockback|GetKockbackDuration))
      (Variables|Knockback|SetKnockbackTimer (+ (Variables|Knockback|GetKnockbackTimer) (Utilities|Time|GetWorldDeltaSeconds)))
      (else
        (Knockback|StopKnockback)))))

(fn StopKnockback
  (Variables|Knockback|SetbKnockback false)
  (Variables|Knockback|SetKnockbackTimer 0.0))

(fn StartDash
  (bind _lookdirection (Variables|Default|GetLookDirection))
  (bind _movementmode (Variables|Movement|GetMovementMode))
  (bind _walldirection (Variables|Wall|GetWallDirection))
  (bind _returnvalue (* _walldirection -1.0))
  (bind _returnvalue_2 (Utilities|Enum|Equal(Enum) _movementmode "NewEnumerator5"))
  (bind _returnvalue_3 (select _returnvalue_2 (Math|Vector|MakeVector 0.0 _returnvalue 0.0) _lookdirection))
  (if (< (Variables|Dash|GetDashCounter) 1)
    (bind _output_get (Variables|Dash|SetDashCounter (+ (stale _output_get) 1)))
    (Variables|Dash|SetDashDirection _returnvalue_3)
    (CallFunction|Look (== (.Y (Math|Vector|BreakVector _returnvalue_3)) 1.0))
    (Movement|ChangeMovement "NewEnumerator4")
    (Utilities|Time|ClearTimerbyFunctionName self "Ungrounded")))

(fn Dashing
  (if (Utilities|Enum|Equal(Enum) (Variables|Movement|GetMovementMode) "NewEnumerator4")
    (Movement|AddVelocity (Variables|Dash|GetDashDirection) (Variables|Dash|GetDashAcceleration))
    (bind _output_get (Variables|Dash|SetDashTimer (+ (Variables|Dash|GetDashTimer) (Utilities|Time|GetWorldDeltaSeconds))))
    (if (>= _output_get (Variables|Dash|GetDashDuration))
      (Variables|Dash|SetDashTimer 0.0)
      (Dash|StopDash))))

(fn StopDash
  (Movement|ChangeMovement "NewEnumerator2"))

(fn Grounded
  (Variables|Default|SetHeight (.z (Transformation|GetActorLocation)))
  (Movement|ChangeMovement "NewEnumerator0")
  (CallFunction|Refresh)
  (Utilities|Time|SetTimerbyFunctionName self "Ungrounded" 1e-06))

(fn Refresh
  (Variables|Dash|SetDashCounter 0)
  (Variables|Jump|SetbDoubleJump true))

(fn LandedWallFalse
  (Variables|Wall|SetbLandedWall false))

(fn CheckWallCollision
  (Utilities|FlowControl|Sequence
    (:then_0
      (for _index (range 0 1)
        (bind _outhit (Collision|SphereTraceForObjects (+ (Transformation|GetActorLocation) (Math|Vector|MakeVector 0.0 (Utilities|Select :Index _index :Option%200 2e+01 :Option%201 -2e+01) 0.0)) (+ (Transformation|GetActorLocation) (Math|Vector|MakeVector 0.0 (Utilities|Select :Index _index :Option%200 2e+01 :Option%201 -2e+01) 0.0)) 5.0 (Utilities|Array|MakeArray "ObjectTypeQuery1" "ObjectTypeQuery2") false 0 "None"))
        (if (.bblockinghit _outhit)
          (if (> (Math|Float|Absolute(Float) (Math|Vector|DotProduct (.normal _outhit) "0,1.000000, 0")) 0.71)
            (Variables|Wall|SetbTouchingWall true)
            (Variables|Wall|SetWallDirection (Math|Float|Sign(Float) (* (.Y (Math|Vector|BreakVector (.normal _outhit))) -1.0)))
            (CallFunction|Refresh)
            (return)))))
    (:then_1
      (Variables|Wall|SetbTouchingWall false)
      (return))))